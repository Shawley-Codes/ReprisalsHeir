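; Fireball projectile actor that damages enemies it overlaps and destroys itself after a short fixed lifetime.
; On overlap it tries a cast to BP_enemy, then CharherEnemy, and passes its Damage variable to that class's TakeDamage, without destroying itself.
; A separate SetISpeed event sets the projectile movement's initial speed.
; An older name-based hit check with debug prints and destruction is left unconnected.
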(event Custom|SetISpeed
  (Variables|/Script/Engine.ProjectileMovementComponent|SetInitialSpeed (Variables|Components|GetProjectileMovement1) 1e+03))

(event Collision|EventActorBeginOverlap
  (params (OtherActor :type Actor%20Object%20Reference))
  (bind _asbp_enemy (Utilities|Casting|CastToBP_enemy OtherActor)
    (:then
      (Default|TakeDamage _asbp_enemy (Variables|Default|GetDamage)))
    (:CastFailed
      (bind _ascharher_enemy (Utilities|Casting|CastToCharherEnemy OtherActor))
      (Default|TakeDamage _ascharher_enemy (Variables|Default|GetDamage)))))

(event EventBeginPlay
  (Utilities|FlowControl|Delay 5.0)
  (Actor|DestroyActor))

(fn ConstructionScript)