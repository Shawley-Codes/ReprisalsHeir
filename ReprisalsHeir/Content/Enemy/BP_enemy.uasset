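; Spider enemy that damages the player and can itself be damaged and destroyed.
; The construction script tints the mesh's body and eye glow by spider type.
; DamageTrigger overlap hurts FirstPersonCharacter after a short delay, without rechecking the overlap, while TakeDamage lowers HP or destroys the enemy when damage is lethal.
; Old fireball/sword hit detection and death montage logic remain disconnected, and mesh overlaps only print the other actor's name.
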(event OnComponentBeginOverlap(CapsuleComponent)
  (params (OverlappedComponent :type Primitive%20Component%20Object%20Reference) (OtherActor :type Actor%20Object%20Reference) (OtherComp :type Primitive%20Component%20Object%20Reference) (OtherBodyIndex :type Integer) (bFromSweep :type Boolean) (SweepResult :type Hit%20Result%20Structure%20%28by%20ref%29)))

(event OnComponentBeginOverlap(Mesh)
  (params (OverlappedComponent :type Primitive%20Component%20Object%20Reference) (OtherActor :type Actor%20Object%20Reference) (OtherComp :type Primitive%20Component%20Object%20Reference) (OtherBodyIndex :type Integer) (bFromSweep :type Boolean) (SweepResult :type Hit%20Result%20Structure%20%28by%20ref%29))
  (Development|PrintString (Utilities|GetDisplayName OtherActor)))

(event OnComponentBeginOverlap(DamageTrigger)
  (params (OverlappedComponent :type Primitive%20Component%20Object%20Reference) (OtherActor :type Actor%20Object%20Reference) (OtherComp :type Primitive%20Component%20Object%20Reference) (OtherBodyIndex :type Integer) (bFromSweep :type Boolean) (SweepResult :type Hit%20Result%20Structure%20%28by%20ref%29))
  (bind _asfirst_person_character (Utilities|Casting|CastToFirstPersonCharacter OtherActor))
  (Utilities|FlowControl|Delay 0.7)
  (Utilities|IsValid _asfirst_person_character
    (:Is%20Valid
      (Default|TakeDamage _asfirst_person_character (Math|Float|Truncate (Variables|Default|GetDamage))))))

(event EventBeginPlay)

(event Collision|EventActorBeginOverlap
  (params (OtherActor :type Actor%20Object%20Reference))
  ;[1 1 1] Old Damage Code
)

(event EventTick
  (params (DeltaSeconds :type Float%20%28single-precision%29)))

(fn ConstructionScript
  (bind _mesh (Variables|Character|GetMesh))
  (Utilities|FlowControl|Sequence
    (:then_0
      (switch Utilities|FlowControl|Switch|SwitchonEnum_TypeOfEnemy (Variables|Default|GetTypeOfEnemy)
        (:NewEnumerator0
          (Rendering|Material|SetVectorParameterValueonMaterials _mesh "BodyGlow" "1.000000,1.000000,1.000000")
          (Rendering|Material|SetVectorParameterValueonMaterials _mesh "EyeGlow" "1.000000,1.000000,1.000000"))
        (:NewEnumerator1
          (Rendering|Material|SetVectorParameterValueonMaterials _mesh "BodyGlow" "1.000000, 0, 0")
          (Rendering|Material|SetVectorParameterValueonMaterials _mesh "EyeGlow" "1.000000, 0, 0"))
        (:NewEnumerator2
          (Rendering|Material|SetVectorParameterValueonMaterials _mesh "BodyGlow" "0, 0,1.000000")
          (Rendering|Material|SetVectorParameterValueonMaterials _mesh "EyeGlow" "0, 0,1.000000"))
        (:NewEnumerator3
          (Rendering|Material|SetVectorParameterValueonMaterials _mesh "BodyGlow" "0.000000,1.000000, 0")
          (Rendering|Material|SetVectorParameterValueonMaterials _mesh "EyeGlow" "0.000000,1.000000, 0"))
        (:NewEnumerator4
          (Rendering|Material|SetVectorParameterValueonMaterials _mesh "BodyGlow" "0.750000,0.500000,0.250000")
          (Rendering|Material|SetVectorParameterValueonMaterials _mesh "EyeGlow" "0.250000,0.500000,0.750000"))))))

(fn TakeDamage
  (params (Damage :type Float%20%28single-precision%29))
  (if (>= Damage (Variables|Default|GetHP))
    (Actor|DestroyActor)
    (else
      (Variables|Default|SetHP (- (Variables|Default|GetHP) Damage)))))