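; BP_Potion is a collectable health potion that heals the player when walked over.
; On overlap it casts to FirstPersonCharacter, confirms it is the player pawn, and passes through a DoOnce.
; It adds a fixed amount to the character's health, setting a hardcoded 100 when the sum reaches MaxHealth, then destroys itself.
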(event EventBeginPlay)

(event EventTick
  (params (DeltaSeconds :type Float%20%28single-precision%29)))

(event Collision|EventActorBeginOverlap
  (params (OtherActor :type Actor%20Object%20Reference))
  ;[1 1 1] Collectables Overlap Trigger and Disapear
  (bind _asfirst_person_character (Utilities|Casting|CastToFirstPersonCharacter OtherActor))
  (if (== OtherActor (Game|Player|GetPlayerPawn 0))
    (Utilities|FlowControl|DoOnce false
      (:Completed
        (bind _output_get (Variables|Default|Setplayer _asfirst_person_character))
        (bind (_currenhealth _maxhealth) (Default|GetHealth _output_get))
        (if (>= (+ _currenhealth 20) _maxhealth)
          (Variables|/Game/FirstPersonBP/Blueprints/FirstPersonCharacter.FirstPersonCharacter_C|SetHealth _output_get 100)
          (else
            (Variables|/Game/FirstPersonBP/Blueprints/FirstPersonCharacter.FirstPersonCharacter_C|SetHealth _output_get (+ _currenhealth 20))))
        (Actor|DestroyActor)))))

(fn ConstructionScript)